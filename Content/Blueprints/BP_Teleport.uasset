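; BP_Teleport is a teleporter that moves an overlapping actor to the arrow component of a linked TeleportLocation.
; On overlap it compares the other actor's class display name with that of its Actor reference, printing a mismatch message otherwise.
; On a match it applies SetActorLocation, root SetWorldTransform and Teleport in succession, then prints results.
; An in-graph Dutch note says these methods work for the player but fail for BP_SoccerBall.
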(event `self.ReceiveActorBeginOverlap`
  (params (OtherActor :type "Actor Object Reference"))
  (bind _arrowcomponent (`TargetPoint.ArrowComponent` (`self.TeleportLocation`)))
  (bind _returnvalue (`SceneComponent.K2_GetComponentLocation` _arrowcomponent))
  (bind _returnvalue_2 (`SceneComponent.K2_GetComponentRotation` _arrowcomponent))
  (if (`KismetStringLibrary.EqualEqual_StrStr` (`KismetSystemLibrary.GetClassDisplayName` (`GameplayStatics.GetObjectClass` OtherActor)) (`KismetSystemLibrary.GetClassDisplayName` (`self.Actor`)))
    ;[1 1 1] Geen van deze funties werkt voor de BP_SoccerBall, werkt wel voor de speler
    (bind (_sweephitresult _returnvalue_3) (`self.K2_SetActorLocation` OtherActor _returnvalue false true))
    (`SceneComponent.K2_SetWorldTransform` (`Actor.RootComponent` OtherActor) (`KismetMathLibrary.MakeTransform` _returnvalue _returnvalue_2) false true)
    (bind _returnvalue_4 (`self.K2_TeleportTo` OtherActor _returnvalue _returnvalue_2))
    (`KismetSystemLibrary.PrintString` (`KismetStringLibrary.Concat_StrStr` "Successfully teleported: " (`KismetStringLibrary.Conv_BoolToString` _returnvalue_3) " Second check: " (`KismetStringLibrary.Conv_BoolToString` _returnvalue_4)))
    (else
      (`KismetSystemLibrary.PrintString` "Object not match" true true (struct :`R` 1.0 :`B` 0.694075 :`A` 1.0)))))

(fn `UserConstructionScript`)